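; BP_ChickenTame is an ambient chicken character that wanders at random through the level and clucks.
; BeginPlay randomizes its yaw, then starts WalkRandom, a self-restarting loop that waits, randomizes walk speed, plays the walk animation and uses AIMoveTo toward nearby navmesh coordinates.
; Success and failure both stop the animation and restart the loop.
; Noise plays one cluck after a random delay; its trailing delay leads nowhere, so the sound never repeats.
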(event Custom|Noise
  ;[1 1 1] Chicken Noise
  (Utilities|IsValid self
    (:Is%20Valid
      (Utilities|FlowControl|Delay (Math|Random|RandomFloatinRange 1.0 25.0))
      (Audio|PlaySoundatLocation "/Game/Sounds/Cue/chickin_noise_cue.chickin_noise_cue" (Transformation|GetWorldLocation (Variables|Collision|GetCapsuleComponent)) "0, 0, 0" 1.0 1.0 0.0 0 0 0 0)
      (Utilities|FlowControl|Delay (Math|Random|RandomFloatinRange 25.0 5e+01)))))

(event Custom|WalkRandom
  (bind _returnvalue (Transformation|GetActorLocation))
  (bind _randomlocation (AI|Navigation|GetRandomReachablePointinRadius _returnvalue 3e+02 0 0))
  ;[1 1 1] Idle Random Movement
  (Utilities|FlowControl|Delay (Math|Random|RandomFloatinRange 1.0 1e+01))
  (Variables|/Script/Engine.CharacterMovementComponent|SetMaxWalkSpeed (Variables|Character|GetCharacterMovement) (Math|Random|RandomFloatinRange 5e+01 2e+02))
  (Components|Animation|PlayAnimation (Variables|Character|GetMesh) "/Game/Level/ChickenRun_Assets/Chickin/Anim/chicken_walk.chicken_walk" true)
  (AI|AIMoveTo self (Math|Vector|MakeVector (.x _randomlocation) (.y _randomlocation) (.Z (Class|KismetMathLibrary|BreakVector3f _returnvalue))) 0 5.0 false
    (:OnSuccess
      _)
    (:OnFail
      _))
  (Audio|Components|Audio|Stop (Variables|Character|GetMesh))
  (CallFunction|WalkRandom))

(event EventBeginPlay
  ;[1 1 1] Set random spawn rotation
  (Transformation|SetActorRotation (Math|Rotator|MakeRotator 0.0 0.0 (Math|Random|RandomFloatinRange 0.0 359.0)))
  (CallFunction|WalkRandom)
  (CallFunction|Noise))

(event EventTick
  (params (DeltaSeconds :type Float%20%28single-precision%29)))

(fn ConstructionScript)