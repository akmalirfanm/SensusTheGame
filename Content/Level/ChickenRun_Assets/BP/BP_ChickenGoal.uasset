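; BP_ChickenGoal is a goal zone in the ChickenRun level that removes chickens entering its trigger box.
; On overlap with a BP_Chicken, it plays two sounds at the chicken's location, briefly blinks the cube's opacity, then destroys the chicken after the short delay.
; The construction script gives the cube a dynamic instance of the goal-mark material to support the blink.
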(event OnComponentBeginOverlap(TriggerBox)
  (params (OverlappedComponent :type Primitive%20Component%20Object%20Reference) (OtherActor :type Actor%20Object%20Reference) (OtherComp :type Primitive%20Component%20Object%20Reference) (OtherBodyIndex :type Integer) (bFromSweep :type Boolean) (SweepResult :type Hit%20Result%20Structure%20%28by%20ref%29))
  (bind _cube (Variables|Default|GetCube))
  ;[1 1 1] Overlapping with chicken
  (bind _asbp_chicken (Utilities|Casting|CastToBP_Chicken OtherActor))
  ;[1 1 1] Play sound at overlapping area
  (Audio|PlaySoundatLocation "/Game/Sounds/chickengoal_Cue.chickengoal_Cue" (Transformation|GetWorldLocation (Variables|/Script/Engine.Character|GetCapsuleComponent _asbp_chicken)) "0, 0, 0" 1.0 1.0 0.0 0 0 0 0)
  (Audio|PlaySoundatLocation "/Game/Interface_And_Item_Sounds/Cues/Pop_09_Cue.Pop_09_Cue" (Transformation|GetWorldLocation (Variables|/Script/Engine.Character|GetCapsuleComponent _asbp_chicken)) "0, 0, 0" 1.0 1.0 0.0 0 0 0 0)
  ;[1 1 1] Blink effect on cube
  (Rendering|Material|SetScalarParameterValueonMaterials _cube "Opacity" 0.3)
  (Utilities|FlowControl|Delay 0.2)
  (Rendering|Material|SetScalarParameterValueonMaterials _cube "Opacity" 0.15)
  ;[1 1 1] Destroy chicken from level :(
  (Actor|DestroyActor _asbp_chicken))

(event EventBeginPlay)

(event Collision|EventActorBeginOverlap
  (params (OtherActor :type Actor%20Object%20Reference)))

(event EventTick
  (params (DeltaSeconds :type Float%20%28single-precision%29)))

(fn ConstructionScript
  (Rendering|Material|CreateDynamicMaterialInstance (Variables|Default|GetCube) 0 "/Game/Level/ChickenRun_Assets/BP/M_GoalMark.M_GoalMark" "None" :!class /Script/Engine.PrimitiveComponent))