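; Chicken character that idly wanders and flees from the player's third-person character.
; A TriggerRun overlap toggles fleeing, which speeds it up, loops the walk animation and moves it via AIMoveTo to a random reachable point away from the player.
; Otherwise it makes short, slow random moves after random pauses.
; Tick drives both behaviors and occasional clucking, relying on random Delays to space out wandering and sounds.
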(event OnComponentBeginOverlap(TriggerRun)
  (params (OverlappedComponent :type Primitive%20Component%20Object%20Reference) (OtherActor :type Actor%20Object%20Reference) (OtherComp :type Primitive%20Component%20Object%20Reference) (OtherBodyIndex :type Integer) (bFromSweep :type Boolean) (SweepResult :type Hit%20Result%20Structure%20%28by%20ref%29))
  ;[1 1 1] Set event when overlapping with player
  (Utilities|Casting|CastToBP_ThirdPersonCharacter OtherActor)
  (Variables|Default|SetisIdle? false)
  (Variables|Default|SetisOverlapping? true))

(event OnComponentEndOverlap(TriggerRun)
  (params (OverlappedComponent :type Primitive%20Component%20Object%20Reference) (OtherActor :type Actor%20Object%20Reference) (OtherComp :type Primitive%20Component%20Object%20Reference) (OtherBodyIndex :type Integer))
  ;[1 1 1] Set event when overlapping with player
  (Utilities|Casting|CastToBP_ThirdPersonCharacter OtherActor)
  (Variables|Default|SetisOverlapping? false))

(event Custom|Noise
  ;[1 1 1] Chicken Noise
  (Utilities|IsValid self
    (:Is%20Valid
      (Utilities|FlowControl|Delay (Math|Random|RandomFloatinRange 1.0 25.0))
      (Audio|PlaySoundatLocation "/Game/Sounds/Cue/chickin_noise_cue.chickin_noise_cue" (Transformation|GetWorldLocation (Variables|Collision|GetCapsuleComponent)) "0, 0, 0" 1.0 1.0 0.0 0 0 0 0)
      (Utilities|FlowControl|Delay (Math|Random|RandomFloatinRange 25.0 5e+01)))))

(event Custom|ChickinRun
  (bind _returnvalue (Game|GetPlayerCharacter 0))
  (bind _returnvalue_2 (Transformation|GetActorLocation))
  (bind _capsulecomponent (Variables|/Script/Engine.Character|GetCapsuleComponent _returnvalue))
  (bind _returnvalue_3 (Transformation|GetWorldLocation _capsulecomponent))
  (bind _returnvalue_4 (Math|Rotator|FindLookatRotation _returnvalue_2 _returnvalue_3))
  (bind _returnvalue_5 (Math|Vector|GetForwardVector _returnvalue_4))
  (bind _returnvalue_6 (* _returnvalue_5 -5e+02))
  (bind _returnvalue_7 (+ _returnvalue_2 _returnvalue_6))
  (bind (_x _y) (Math|Vector|BreakVector _returnvalue_7))
  ;[1 1 1] Run Awawy
  (if (Variables|Default|GetisOverlapping?)
    (Variables|/Script/Engine.CharacterMovementComponent|SetMaxWalkSpeed (Variables|Character|GetCharacterMovement) (Math|Random|RandomFloatinRange 6.1e+02 6.5e+02))
    (Components|Animation|PlayAnimation (Variables|Character|GetMesh) "/Game/Level/ChickenRun_Assets/Chickin/Anim/chicken_walk.chicken_walk" true)
    (AI|AIMoveTo self (.RandomLocation (AI|Navigation|GetRandomReachablePointinRadius (Math|Vector|MakeVector _x _y (.Z (Math|Vector|BreakVector _returnvalue_2))) 4e+02 0 0)) 0 5.0 false
      (:OnSuccess
        _)
      (:OnFail
        _))
    (Audio|Components|Audio|Stop (Variables|Character|GetMesh))))

(event Custom|WalkRandom
  (bind _returnvalue (Transformation|GetActorLocation))
  (bind _randomlocation (AI|Navigation|GetRandomReachablePointinRadius _returnvalue 1e+02 0 0))
  ;[1 1 1] Idle Random Movement
  (if (not (Variables|Default|GetisOverlapping?))
    (Audio|Components|Audio|Stop (Variables|Character|GetMesh))
    (Utilities|FlowControl|Delay (Math|Random|RandomFloatinRange 2.0 6.0))
    (Variables|/Script/Engine.CharacterMovementComponent|SetMaxWalkSpeed (Variables|Character|GetCharacterMovement) (Math|Random|RandomFloatinRange 5e+01 2e+02))
    (AI|AIMoveTo self (Math|Vector|MakeVector (.x _randomlocation) (.y _randomlocation) (.Z (Class|KismetMathLibrary|BreakVector3f _returnvalue))) 0 5.0 false)))

(event EventBeginPlay
  ;[1 1 1] Set random spawn rotation
  (Transformation|SetActorRotation (Math|Rotator|MakeRotator 0.0 0.0 (Math|Random|RandomFloatinRange 0.0 359.0))))

(event EventTick
  (params (DeltaSeconds :type Float%20%28single-precision%29))
  (CallFunction|Noise)
  (Utilities|FlowControl|Sequence
    (:then_0
      (if (Variables|Default|GetisOverlapping?)
        (CallFunction|ChickinRun)))
    (:then_1
      (CallFunction|WalkRandom))))

(fn ConstructionScript)