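; BP_FarmTile is a farm tile that grows a crop from the seed selected on BP_ThirdPersonCharacter when Plant is called on an unplanted tile.
; Seed 0 starts PlantingPlant1, which swaps three static mesh stages, with a timed wait between each, then marks the crop fully grown and harvestable as Plant1.
; The GrowTime macro runs each wait as a one-second Delay loop that shows the remaining time on a Text3D countdown.
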(event Custom|PlantingPlant1
  (bind _relativetransformlocation (Variables|Default|GetRelativeTransformLocation))
  (bind _returnvalue (AddComponent|AddStaticMeshComponent false (Math|Transform|MakeTransform _relativetransformlocation "0, 0, 0" "1.000000,1.000000,1.000000")))
  (Utilities|GrowTime (Variables|Default|GetPlant1GrowTime)
    (:Out
      (Components|DestroyComponent _returnvalue)
      (bind _returnvalue_2 (AddComponent|AddStaticMeshComponent false (Math|Transform|MakeTransform _relativetransformlocation "0, 0, 0" "1.000000,1.000000,1.000000")))
      (Utilities|GrowTime (Variables|Default|GetPlant1GrowTime)
        (:Out
          (Components|DestroyComponent _returnvalue_2)
          (bind _returnvalue_3 (AddComponent|AddStaticMeshComponent false (Math|Transform|MakeTransform _relativetransformlocation "0, 0, 0" "1.000000,1.000000,1.000000")))
          (Variables|Default|SetFullyGrow? true)
          (Variables|Default|SetCurrentMesh _returnvalue_3)
          (Variables|Default|SetWhatCanBeHarvested? "Plant1"))))))

(event EventPlant
  (if (not (Variables|Default|GetIsPlanted?))
    (bind _asbp_third_person_character (Utilities|Casting|CastToBP_ThirdPersonCharacter (Game|GetPlayerCharacter 0)))
    (switch int (Variables|/Game/ThirdPerson/Blueprints/BP_ThirdPersonCharacter.BP_ThirdPersonCharacter_C|GetSeed _asbp_third_person_character)
      (:0
        (CallFunction|PlantingPlant1)
        (Variables|Default|SetIsPlanted? true)))))

(event EventBeginPlay
  (Class|Text3DComponent|SetText (Variables|Default|GetText3D) (Variables|Default|GetValue)))

(fn ConstructionScript)