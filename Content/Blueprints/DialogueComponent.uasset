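; Dialogue component that runs a conversation as a behavior tree when the player interacts with it.
; BeginPlay spawns a dedicated DialogueAIController to drive the tree.
; OnInteraction shows a DialogWidget, switches to UI-only input with the cursor visible, starts DialogTree and passes the widget through DialogBlackboard.
; The widget's exit event stops the tree, removes the widget and restores game input.
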(event Custom|onExit_Event_0
  (bind _dialogwidget (Variables|Default|GetDialogWidget))
  (bind _returnvalue (Widget|GetOwningPlayer _dialogwidget))
  (Input|SetInputModeGameOnly _returnvalue)
  (Input|EnableInput (Game|GetPlayerCharacter 0) (Game|GetPlayerController 0))
  (Variables|/Script/Engine.PlayerController|SetbShowMouseCursor _returnvalue false)
  (AI|Logic|StopLogic (Variables|/Script/AIModule.AIController|GetBrainComponent (Variables|Default|GetAIController)) "Dialog Exited")
  (Widget|RemovefromParent (Variables|Default|GetDialogWidget)))

(event EventBeginPlay
  (bind _returnvalue (Game|SpawnActorfromClass "/Game/Blueprints/DialogueAIController.DialogueAIController_C" (Math|Transform|MakeTransform "0, 0, 0" "0, 0, 0" "1.000000,1.000000,1.000000") "Undefined" 0 0))
  (Variables|Default|SetAIController _returnvalue))

(event EventOnInteraction
  (params (PlayerCharacter :type BP%20Third%20Person%20Character%20Object%20Reference))
  (bind _returnvalue (Pawn|GetController PlayerCharacter))
  (bind _asplayer_controller (Utilities|Casting|CastToPlayerController _returnvalue))
  (bind _returnvalue_2 (UserInterface|CreateWidget "/Game/Widgets/DialogWidget.DialogWidget_C" _asplayer_controller))
  (bind _output_get (Variables|Default|SetDialogWidget _returnvalue_2))
  (EventDispatchers|AssignOnExit _output_get (delegate Custom|onExit_Event_0))
  (UserInterface|Viewport|AddtoViewport _output_get 0)
  (Input|SetInputModeUIOnly _asplayer_controller _output_get "DoNotLock")
  ;[1 1 1] disable input
  (Input|DisableInput (Game|GetPlayerCharacter 0) (Game|GetPlayerController 0))
  (Variables|/Script/Engine.PlayerController|SetbShowMouseCursor _asplayer_controller true)
  (AI|RunBehaviorTree (Variables|Default|GetAIController) (Variables|Default|GetDialogTree))
  (bind _blackboardcomponent (Class|AIController|UseBlackboard (Variables|Default|GetAIController) "/Game/Blueprints/DialogBlackboard.DialogBlackboard"))
  (AI|Components|Blackboard|SetValueasObject _blackboardcomponent (Utilities|Name|MakeLiteralName "DialogWidget") (Variables|Default|GetDialogWidget)))