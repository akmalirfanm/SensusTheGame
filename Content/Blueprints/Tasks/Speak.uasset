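; Behavior tree task that makes a dialog widget speak a line of text.
; On execute it reads the DialogWidget object from the blackboard, binds to its OnChatFinished event and calls Speak with the Text variable.
; The task stays running until the chat finishes, then unbinds the event and finishes with success.
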(event Custom|OnChatFinished
  (EventDispatchers|UnbindEventfromOnChatFinished (.AsDialog%20Widget (Utilities|Casting|CastToDialogWidget (Class|BTFunctionLibrary|GetBlackboardValueasObject (Variables|Default|GetDialogWidget)))) (delegate Custom|OnChatFinished))
  (AI|BehaviorTree|FinishExecute true))

(event EventReceiveExecuteAI
  (params (OwnerController :type AI%20Controller%20Object%20Reference) (ControlledPawn :type Pawn%20Object%20Reference))
  (bind _dialogwidget (Variables|Default|GetDialogWidget))
  (bind _returnvalue (Class|BTFunctionLibrary|GetBlackboardValueasObject _dialogwidget))
  (bind _asdialog_widget (Utilities|Casting|CastToDialogWidget _returnvalue))
  (EventDispatchers|AssignOnChatFinished _asdialog_widget (EventDispatchers|CreateEvent :!event Custom|OnChatFinished))
  (Default|Speak _asdialog_widget (Variables|Default|GetText)))