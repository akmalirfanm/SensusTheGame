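; BP_NPC_official_male_0 is a male official NPC that shows a text prompt when the player is nearby and can play a meeting-speaker animation.
; Box overlap events cast to BP_ThirdPersonCharacter, then show the TextRender on entry and hide it on exit.
; A separate PlayAnim event, not called within this Blueprint, plays the discussion animation once on the Mesh.
; BeginPlay, the construction script and PassVar are empty.
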(event OnComponentBeginOverlap(Box)
  (params (OverlappedComponent :type Primitive%20Component%20Object%20Reference) (OtherActor :type Actor%20Object%20Reference) (OtherComp :type Primitive%20Component%20Object%20Reference) (OtherBodyIndex :type Integer) (bFromSweep :type Boolean) (SweepResult :type Hit%20Result%20Structure%20%28by%20ref%29))
  (Utilities|Casting|CastToBP_ThirdPersonCharacter OtherActor)
  (Development|SetHiddeninGame (Variables|Default|GetTextRender) false false))

(event OnComponentEndOverlap(Box)
  (params (OverlappedComponent :type Primitive%20Component%20Object%20Reference) (OtherActor :type Actor%20Object%20Reference) (OtherComp :type Primitive%20Component%20Object%20Reference) (OtherBodyIndex :type Integer))
  (Utilities|Casting|CastToBP_ThirdPersonCharacter OtherActor)
  (Development|SetHiddeninGame (Variables|Default|GetTextRender) true false))

(event EventBeginPlay)

(event EventPlayAnim
  (Components|Animation|PlayAnimation (Variables|Character|GetMesh) "/Game/Characters/NPC/Animation/meeting_speaker_discuss_f_270764_meeting_speaker_discuss_f_270764fix.meeting_speaker_discuss_f_270764_meeting_speaker_discuss_f_270764fix" false))

(fn ConstructionScript)

(fn PassVar
  (return))