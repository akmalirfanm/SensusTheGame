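; Official male NPC that the player talks to, with idle and speaking animations and a distance-labelled waypoint marker.
; Dialogue starts disabled until WaypointVisibility shows the marker and enables the first tree; EndDialog switches trees by DialogIndex.
; Box overlap by the player shows interact text and hides the marker.
; Tick updates the distance and smoothly turns the NPC toward the player during dialogue, then back to its starting rotation.
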(event OnComponentBeginOverlap(Box)
  (params (OverlappedComponent :type Primitive%20Component%20Object%20Reference) (OtherActor :type Actor%20Object%20Reference) (OtherComp :type Primitive%20Component%20Object%20Reference) (OtherBodyIndex :type Integer) (bFromSweep :type Boolean) (SweepResult :type Hit%20Result%20Structure%20%28by%20ref%29))
  ;[1 1 1] Spawn interact text above and disable waypoint
  (Utilities|Casting|CastToBP_ThirdPersonCharacter OtherActor)
  (Development|SetHiddeninGame (Variables|Default|GetTextRender) false false)
  (Rendering|SetVisibility (Variables|Default|GetWaypoint) false false))

(event OnComponentEndOverlap(Box)
  (params (OverlappedComponent :type Primitive%20Component%20Object%20Reference) (OtherActor :type Actor%20Object%20Reference) (OtherComp :type Primitive%20Component%20Object%20Reference) (OtherBodyIndex :type Integer))
  ;[1 1 1] Spawn interact text above and disable waypoint
  (Utilities|Casting|CastToBP_ThirdPersonCharacter OtherActor)
  (Development|SetHiddeninGame (Variables|Default|GetTextRender) true false))

(event EventEndDialog
  ;[1 1 1] Change Dialog Tree Set
  (Variables|Default|SetisLooking? false)
  (Components|Animation|PlayAnimation (Variables|Character|GetMesh) "/Game/Characters/NPC/official_male_1/idle_male.idle_male" true)
  (if (<= (Variables|Default|GetDialogIndex) 1)
    (bind _result (Math|Integer|IncrementInt (Variables|Default|GetDialogIndex))
      (:%20%20
        (bind _output_get (Variables|Default|SetDialogIndex _result))
        (switch int _output_get
          (:Default
            (Variables|/Game/Blueprints/DialogueComponent.DialogueComponent_C|SetDialogTree (Variables|Default|GetDialogueComponent) (Variables|Default|GetDialog%20Tree%201) :!label _label))
          (:0
            (goto _label))
          (:1
            (Variables|/Game/Blueprints/DialogueComponent.DialogueComponent_C|SetDialogTree (Variables|Default|GetDialogueComponent) (Variables|Default|GetDialog%20Tree%202))))))))

(event EventBeginPlay
  ;[1 1 1] Initialize DialogComponent
  (Variables|/Game/Blueprints/DialogueComponent.DialogueComponent_C|SetDialogTree (Variables|Default|GetDialogueComponent) (Variables|Default|GetDialogDisable))
  (Rendering|SetVisibility (Variables|Default|GetWaypoint) false false)
  (Components|Animation|PlayAnimation (Variables|Default|GetVroid) "/Game/Characters/NPC/official_male_1/idle_male.idle_male" true)
  (Variables|Default|SetDefaultRotation (Transformation|GetWorldRotation (Variables|Collision|GetCapsuleComponent))))

(event EventWaypointVisibility
  ;[1 1 1] Set Marker and Enable Dialog
  (Rendering|SetVisibility (Variables|Default|GetWaypoint) true false)
  (Variables|/Game/Blueprints/DialogueComponent.DialogueComponent_C|SetDialogTree (Variables|Default|GetDialogueComponent) (Variables|Default|GetDialog%20Tree%201)))

(event EventPlayAnim
  ;[1 1 1] Play animation when speaking
  (Development|SetHiddeninGame (Variables|Default|GetTextRender) true false)
  (Variables|Default|SetisLooking? true)
  (if (not (Variables|Default|GetisAnimPlaying?))
    (Variables|Default|SetisAnimPlaying? true)
    (Components|Animation|PlayAnimation (Variables|Character|GetMesh) "/Game/Characters/NPC/official_male_1/speak_male.speak_male" false)
    (Utilities|FlowControl|Delay 4.0)
    (Variables|Default|SetisAnimPlaying? false)))

(event EventTick
  (params (DeltaSeconds :type Float%20%28single-precision%29))
  (bind _capsulecomponent (Variables|Collision|GetCapsuleComponent))
  (bind _returnvalue (Transformation|GetWorldRotation _capsulecomponent))
  ;[1 1 1] Update marker distance
  (Class|BPIMasterWidget|UpdateDistance(Message) (UserInterface|GetUserWidgetObject (Variables|Default|GetWaypoint)) (Utilities|Text|ToText(String) (Utilities|String|Append (Utilities|String|ToString(Integer) (Math|Float|Truncate (/ (Math|Vector|Distance(Vector) (Transformation|GetActorLocation) (Transformation|GetActorLocation (Game|GetPlayerCharacter 0))) 1e+02))) "m")))
  ;;[1 1 1] Actor Rotator
  (if (Variables|Default|GetisLooking?)
    (Transformation|SetWorldRotation (Variables|Collision|GetCapsuleComponent) (Math|Interpolation|RInterpTo _returnvalue (Math|Rotator|FindLookatRotation (Transformation|GetWorldLocation _capsulecomponent) (Transformation|GetWorldLocation (Variables|/Script/Engine.Character|GetCapsuleComponent (Game|GetPlayerCharacter 0)))) DeltaSeconds 5.0) false false)
    (else
      (Transformation|SetWorldRotation (Variables|Collision|GetCapsuleComponent) (Math|Interpolation|RInterpTo _returnvalue (Variables|Default|GetDefaultRotation) DeltaSeconds 5.0) false false))))

(fn ConstructionScript)